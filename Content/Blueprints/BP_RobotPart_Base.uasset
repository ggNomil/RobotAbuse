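; Base actor for robot parts that can be picked up, outlined with an overlay material while the cursor hovers over the mesh.
; On BeginPlay it binds to OnPickedUp; pickup limits collision to blocking GameTraceChannel1 and calls DetachHelper, while release blocks all channels except that one, which overlaps.
; DetachHelper re-enables physics and gravity and detaches the actor, while AttachmentHelper switches both off.
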(event `self.ReceiveBeginPlay`
  (add `self.OnPickedUp` (`|CreateDelegate` :!event `PickUpEvent`)))

(event `PickUpEvent` :!signature `self.OnPickedUp`
  (params (bPickedUp :type Boolean) (PartType :type "ERobotPartType Enum" :default "None") (RobotPart :type "RobotPart Object Reference"))
  (bind _meshref (`self.MeshRef`))
  (if bPickedUp
    (`PrimitiveComponent.SetCollisionResponseToAllChannels` _meshref "ECR_Ignore")
    (`PrimitiveComponent.SetCollisionResponseToChannel` _meshref "ECC_GameTraceChannel1" "ECR_Block")
    (`self.DetachHelper`)
    (else
      (`PrimitiveComponent.SetCollisionResponseToAllChannels` _meshref "ECR_Block")
      (`PrimitiveComponent.SetCollisionResponseToChannel` _meshref "ECC_GameTraceChannel1" "ECR_Overlap"))))

(event `self.MeshRef.OnBeginCursorOver`
  (params (TouchedComponent :type "PrimitiveComponent Object Reference"))
  (`MeshComponent.SetOverlayMaterial` (`self.MeshRef`) "/Game/Assets/M_Outline.M_Outline"))

(event `self.MeshRef.OnEndCursorOver`
  (params (TouchedComponent :type "PrimitiveComponent Object Reference"))
  (`MeshComponent.SetOverlayMaterial` (`self.MeshRef`) null))

(fn `AttachmentHelper`
  (bind _meshref (`self.MeshRef`))
  (`PrimitiveComponent.SetEnableGravity` _meshref false)
  (`PrimitiveComponent.SetSimulatePhysics` _meshref false))

(fn `DetachHelper`
  (bind _meshref (`self.MeshRef`))
  (`PrimitiveComponent.SetEnableGravity` _meshref true)
  (`PrimitiveComponent.SetSimulatePhysics` _meshref true)
  (`self.K2_DetachFromActor` "KeepRelative"))

(fn `UserConstructionScript`)