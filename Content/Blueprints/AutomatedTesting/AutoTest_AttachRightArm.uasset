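; Functional test that checks whether a right arm part attaches to a torso.
; On prepare it disables physics and gravity on the arm mesh, then each tick nudges the arm slightly along world +X.
; Once the torso's ConnectedParts map holds a valid right-arm entry, movement stops and the test finishes as succeeded after a short delay.
; The graph has no failure branch of its own.
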(event `self.ReceivePrepareTest`
  (bind _meshref (`RobotPart.MeshRef` (`self.Arm`)))
  (`PrimitiveComponent.SetSimulatePhysics` _meshref false)
  (`PrimitiveComponent.SetEnableGravity` _meshref false))

(event `self.ReceiveStartTest`)

(event `self.ReceiveTick`
  (params (DeltaSeconds :type "Float (single-precision)"))
  (bind _arm (`self.Arm`))
  (if (`KismetSystemLibrary.IsValid` (`BlueprintMapLibrary.Map_Find` (`/Game/Blueprints/BP_RobotTorso.ConnectedParts` (`self.Torso`)) "ArmRight"))
    (`KismetSystemLibrary.Delay` 1.0)
    (`self.FinishTest` "Succeeded" "Succeeded :: Part Connected")
    (else
      (`self.K2_SetActorLocation` _arm (+ (`self.K2_GetActorLocation` _arm) (0.05 0.0 0.0)) false false))))

(fn `UserConstructionScript`)